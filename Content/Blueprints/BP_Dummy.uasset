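; BP_Dummy is a stealth assassination target that the player can take down from behind.
; An overlap radius shows or hides an assassinate prompt widget as the third-person character enters or leaves it.
; StealthBackAssassin plays the victim half of a paired knife montage, hides the prompt and returns a reference location and actor rotation, presumably to align the attacker.
; A Ragdoll event enables mesh physics after a short delay for the montage.
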(event OnComponentBeginOverlap(AssassinationRadius)
  (params (OverlappedComponent :type Primitive%20Component%20Object%20Reference) (OtherActor :type Actor%20Object%20Reference) (OtherComp :type Primitive%20Component%20Object%20Reference) (OtherBodyIndex :type Integer) (bFromSweep :type Boolean) (SweepResult :type Hit%20Result%20Structure%20%28by%20ref%29))
  ;[1 1 1] Toggle Assassinate Widget (Text)
  (Utilities|Casting|CastToBP_ThirdPersonCharacter OtherActor)
  (Rendering|SetVisibility (Variables|Default|GetAssassinateWidget) true false))

(event OnComponentEndOverlap(AssassinationRadius)
  (params (OverlappedComponent :type Primitive%20Component%20Object%20Reference) (OtherActor :type Actor%20Object%20Reference) (OtherComp :type Primitive%20Component%20Object%20Reference) (OtherBodyIndex :type Integer))
  ;[1 1 1] Toggle Assassinate Widget (Text)
  (Utilities|Casting|CastToBP_ThirdPersonCharacter OtherActor)
  (Rendering|SetVisibility (Variables|Default|GetAssassinateWidget) false false))

(event Custom|Ragdoll
  ;[1 1 1] Ragdoll
  (Utilities|FlowControl|Delay 2.0) ; Gives the animation montage time to play
  (Physics|SetSimulatePhysics (Variables|Character|GetMesh) true))

(event EventBeginPlay)

(event Collision|EventActorBeginOverlap
  (params (OtherActor :type Actor%20Object%20Reference)))

(event EventTick
  (params (DeltaSeconds :type Float%20%28single-precision%29)))

(fn ConstructionScript)

(fn StealthBackAssassin
  (Animation|PlayAnimMontage "/Game/Characters/RPG_Character/Animations/Assassinations/Paired_Knife_Stealth_KidneyAndNeck_Vic_Montage.Paired_Knife_Stealth_KidneyAndNeck_Vic_Montage" 1.0 "None")
  (CallFunction|Ragdoll)
  (Rendering|SetVisibility (Variables|Default|GetAssassinateWidget) false false)
  (return (Transformation|GetWorldLocation (Variables|Default|GetAssassinationReference)) (Transformation|GetActorRotation)))