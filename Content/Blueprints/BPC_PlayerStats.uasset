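; Player stats component that holds current and max health and stamina and shows them on the owning third-person character's HUD.
; UpdateStat adds a delta to the stat chosen by enum, clamps it between zero and its max, and reports whether it is depleted.
; Tick moves display values toward the current ones at a constant rate, then refreshes both bars and the health text.
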(event Custom|InitHUD
  (CallFunction|UpdateHUD))

(event EventBeginPlay
  (bind _asbp_third_person_character (Utilities|Casting|CastToBP_ThirdPersonCharacter (Components|GetOwner)))
  (Variables|Default|SetPlayerCharacterBP _asbp_third_person_character))

(event EventTick
  (params (DeltaSeconds :type Float%20%28single-precision%29))
  (Variables|Default|SetInterpHealth (Math|Interpolation|FInterptoConstant (Variables|Default|GetInterpHealth) (Variables|Default|GetCurrentHealth) DeltaSeconds 6e+01))
  (Variables|Default|SetInterpStamina (Math|Interpolation|FInterptoConstant (Variables|Default|GetInterpStamina) (Variables|Default|GetCurrentStamina) DeltaSeconds 6e+01))
  (CallFunction|UpdateHUD))

(fn UpdateStat
  (params (Stat :type Enum_PlayerStats%20Enum :default "NewEnumerator0") (NewValue :type Float%20%28double-precision%29))
  (bind _currenthealth (Variables|Default|GetCurrentHealth))
  (bind _maxhealth (Variables|Default|GetMaxHealth))
  (bind _maxstamina (Variables|Default|GetMaxStamina))
  (bind _currentstamina (Variables|Default|GetCurrentStamina))
  (bind _maxhealth_2 (Variables|Default|GetMaxHealth))
  (bind _maxstamina_2 (Variables|Default|GetMaxStamina))
  (bind _returnvalue (Utilities|Select :Index Stat :NewEnumerator0 _currenthealth :NewEnumerator1 _maxhealth_2 :NewEnumerator2 _currentstamina :NewEnumerator3 _maxstamina_2))
  (|SetBy-RefVar _returnvalue (Math|Float|Clamp(Float) (+ NewValue _returnvalue) 0.0 (Utilities|Select :Index Stat :NewEnumerator0 _maxhealth :NewEnumerator1 _maxhealth :NewEnumerator2 _maxstamina :NewEnumerator3 _maxstamina)))
  (return (<= _returnvalue 0.0)))

(fn UpdateHUD
  (bind _interphealth (Variables|Default|GetInterpHealth))
  (bind _playercharacterbp (Variables|Default|GetPlayerCharacterBP))
  (bind _hudwidget (Variables|/Game/ThirdPerson/Blueprints/BP_ThirdPersonCharacter.BP_ThirdPersonCharacter_C|GetHUDWidget _playercharacterbp))
  (Progress|SetPercent (Variables|/Game/UI/WP_MainHUD.WP_MainHUD_C|GetHealthBar _hudwidget) (/ _interphealth (Variables|Default|GetMaxHealth)))
  (Rendering|Components|TextRender|SetText (Variables|/Game/UI/WP_MainHUD.WP_MainHUD_C|GetHealthText _hudwidget) (Utilities|Text|ToText(Integer) (Math|Float|Round _interphealth))) ; This sets the text label on the health bar to the current health value
  (Progress|SetPercent (Variables|/Game/UI/WP_MainHUD.WP_MainHUD_C|GetStaminaBar (Variables|/Game/ThirdPerson/Blueprints/BP_ThirdPersonCharacter.BP_ThirdPersonCharacter_C|GetHUDWidget (Variables|Default|GetPlayerCharacterBP))) (/ (Variables|Default|GetInterpStamina) (Variables|Default|GetMaxStamina))))