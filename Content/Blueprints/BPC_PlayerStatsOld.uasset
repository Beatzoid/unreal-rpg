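; Actor component that tracks health and stamina for the third-person character, caching its owner on BeginPlay.
; Functions raise maximums and adjust current values, with increases capped at the maximum and decreases returning whether the value is depleted.
; Only DecreaseHealth updates the HUD health bar through the cached character.
; DecreaseStamina subtracts current stamina from the depleted amount, reversing the operand order used for health.
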(event EventBeginPlay
  (bind _asbp_third_person_character (Utilities|Casting|CastToBP_ThirdPersonCharacter (Components|GetOwner)))
  (Variables|Default|SetPlayerCharacterBP _asbp_third_person_character))

(fn ConstructionScript)

(fn DecreaseHealth
  (params (Damage :type Float%20%28double-precision%29))
  (bind _output_get (Variables|Health|SetCurrentHealth (- (Variables|Health|GetCurrentHealth) Damage)))
  (Progress|SetPercent (Variables|/Game/UI/WP_MainHUD.WP_MainHUD_C|GetHealthBar (Variables|/Game/ThirdPerson/Blueprints/BP_ThirdPersonCharacter.BP_ThirdPersonCharacter_C|GetHUDWidget (Variables|Default|GetPlayerCharacterBP))) (/ _output_get (Variables|Health|GetMaxHealth)))
  (return (<= (Variables|Health|GetCurrentHealth) 0.0)))

(fn IncreaseMaxHealth
  (params (MaxHealthIncremention :type Float%20%28double-precision%29))
  (Variables|Health|SetMaxHealth (+ (Variables|Health|GetMaxHealth) MaxHealthIncremention)))

(fn IncreaseHealth
  (params (AddedHealth :type Float%20%28double-precision%29))
  (Variables|Health|SetCurrentHealth (+ AddedHealth (Variables|Health|GetCurrentHealth)))
  (if (> (Variables|Health|GetCurrentHealth) (Variables|Health|GetMaxHealth))
    (Variables|Health|SetCurrentHealth (Variables|Health|GetMaxHealth))))

(fn DecreaseStamina
  (params (DepletedStamina :type Float%20%28double-precision%29))
  (Variables|Stamina|SetCurrentStamina (- DepletedStamina (Variables|Stamina|GetCurrentStamina)))
  (return (<= (Variables|Stamina|GetCurrentStamina) 0.0)))

(fn IncreaseMaxStamina
  (params (MaxStaminaIncrease :type Float%20%28double-precision%29))
  (Variables|Stamina|SetMaxStamina (+ MaxStaminaIncrease (Variables|Stamina|GetMaxStamina))))

(fn IncreaseStamina
  (params (StaminaIncrease :type Float%20%28double-precision%29))
  (Variables|Stamina|SetCurrentStamina (Math|Float|Clamp(Float) (+ StaminaIncrease (Variables|Stamina|GetCurrentStamina)) 0.0 (Variables|Stamina|GetMaxStamina))))